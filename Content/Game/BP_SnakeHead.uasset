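; Player-controlled head of a Snake game that moves along the X/Y axes, grows when fed and tracks the score.
; Tick offsets the head by a fraction of its mesh size, then shifts each tail segment into its predecessor's previous location.
; Inputs change direction only when not already moving on that axis, preventing reversals.
; EatFruit increments the score shown in WBP_Main and spawns a scaled-down segment using the head's mesh.
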(event Custom|AddScore
  (bind _result (Math|Integer|IncrementInt (Variables|Default|GetScore))
    (:%20%20
      (Default|SetScore (Variables|Default|GetMainUI) _result))))

(event Custom|AddTail
  (bind _returnvalue (Game|SpawnActorfromClass "/Game/Game/Tail.Tail_C" (Math|Transform|MakeTransform (- (Transformation|GetActorLocation) (* (Variables|Default|GetMoveDir) (Variables|Default|GetStepSize))) "0, 0, 0" "0.600000,0.600000,0.600000") "AlwaysSpawn" 0 0))
  (Components|StaticMesh|SetStaticMesh (Variables|/Game/Game/Trigerable.Trigerable_C|GetMesh _returnvalue) (Variables|/Script/Engine.StaticMeshComponent|GetStaticMesh (Variables|Default|GetHead)))
  (Utilities|Array|Add (Variables|Default|GetTails) _returnvalue))

(event Custom|EatFruit
  (CallFunction|AddScore)
  (CallFunction|AddTail))

(event EventBeginPlay
  (bind _head (Variables|Default|GetHead))
  (bind _staticmesh (Variables|/Script/Engine.StaticMeshComponent|GetStaticMesh _head))
  (bind _returnvalue (StaticMesh|GetBoundingBox _staticmesh))
  (Variables|Default|SetStepSize (- (.x (.max _returnvalue)) (.x (.min _returnvalue))))
  (bind _returnvalue_2 (UserInterface|CreateWidget "/Game/Game/WBP_Main.WBP_Main_C" (Game|GetPlayerController 0)))
  (bind _output_get (Variables|Default|SetMainUI _returnvalue_2))
  (UserInterface|Viewport|AddtoViewport _output_get 0))

(event Collision|EventActorBeginOverlap
  (params (OtherActor :type Actor%20Object%20Reference)))

(event EventTick
  (params (DeltaSeconds :type Float%20%28single-precision%29))
  (Variables|Default|SetActorPreMoveLocation (Transformation|GetActorLocation))
  (Transformation|AddActorWorldOffset (* (Variables|Default|GetMoveDir) (Variables|Default|GetStepSize)))
  (Variables|Default|SetCurrentMoveDir (- (Transformation|GetActorLocation) (Variables|Default|GetActorPreMoveLocation)))
  (for _array_element (Variables|Default|GetTails)
    (bind _output_get (Variables|Default|SetTailCurrentLocation (Transformation|GetActorLocation _array_element)))
    (Transformation|SetActorLocation _array_element (Variables|Default|GetActorPreMoveLocation) false false)
    (Variables|Default|SetActorPreMoveLocation _output_get)))

(event Input|ActionEvents|InputActionMoveUo
  (params (Key :type Key%20Structure :default "None"))
  (:Pressed
    (if (== (.x (Variables|Default|GetCurrentMoveDir)) 0.0)
      (Variables|Default|SetMoveDir "0.500000, 0, 0"))))

(event Input|ActionEvents|InputActionMoveDown
  (params (Key :type Key%20Structure :default "None"))
  (:Pressed
    (if (== (.x (Variables|Default|GetCurrentMoveDir)) 0.0)
      (Variables|Default|SetMoveDir "-0.500000, 0, 0"))))

(event Input|ActionEvents|InputActionMoveLeft
  (params (Key :type Key%20Structure :default "None"))
  (:Pressed
    (if (== (.y (Variables|Default|GetCurrentMoveDir)) 0.0)
      (Variables|Default|SetMoveDir "0,0.500000, 0"))))

(event Input|ActionEvents|InputActionMoveRight
  (params (Key :type Key%20Structure :default "None"))
  (:Pressed
    (if (== (.y (Variables|Default|GetCurrentMoveDir)) 0.0)
      (Variables|Default|SetMoveDir "0,-0.500000, 0"))))

(fn ConstructionScript)